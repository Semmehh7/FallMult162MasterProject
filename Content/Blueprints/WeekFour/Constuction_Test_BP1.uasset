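; A test actor that explodes and changes its static mesh to Car2 when anything begins overlapping its PlayerDetect component.
; The overlap spawns an explosion effect Blueprint at the Scene component's location and enlarges its particle, with no actor filter or one-shot guard.
; The construction script optionally adds an elevated billboard and a randomly colored point light, controlled by the AddSprite and AddPointLight flags.
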(event `self.PlayerDetect.OnComponentBeginOverlap`
  (params (OverlappedComponent :type "PrimitiveComponent Object Reference") (OtherActor :type "Actor Object Reference") (OtherComp :type "PrimitiveComponent Object Reference") (OtherBodyIndex :type Integer) (bFromSweep :type Boolean) (SweepResult :type "HitResult Structure (by ref)"))
  (bind _returnvalue (`|SpawnActorFromClass` "/Game/StarterContent/Blueprints/Blueprint_Effect_Explosion.Blueprint_Effect_Explosion_C" (`KismetMathLibrary.Conv_VectorToTransform` (`SceneComponent.K2_GetComponentLocation` (`self.Scene`))) "Undefined" "MultiplyWithRoot" null null))
  (`SceneComponent.SetWorldScale3D` (`/Game/StarterContent/Blueprints/Blueprint_Effect_Explosion.P_Explosion` _returnvalue) (5.0 5.0 5.0))
  (`StaticMeshComponent.SetStaticMesh` (`self.StaticMesh`) "/Game/Blueprints/WeekTwo/Meshes/Cars/car2.car2"))

(fn `UserConstructionScript`
  ;[1 1 1] Runs when BP is created/spawned
  (if (`self.AddSprite`)
    (`AddComponent|NODE_AddBillboardComponent-0` :`RelativeTransform` (`KismetMathLibrary.MakeTransform` (0.0 0.0 500.0) (struct) (5.0 5.0 5.0))))
  (if (`self.AddPointLight`)
    (bind _returnvalue (`AddComponent|NODE_AddPointLightComponent-0` :`RelativeTransform` (`KismetMathLibrary.MakeTransform` (0.0 0.0 300.0))))
    (`LightComponent.SetLightColor` _returnvalue (`KismetMathLibrary.MakeColor` (`KismetMathLibrary.RandomFloat`) (`KismetMathLibrary.RandomFloat`) (`KismetMathLibrary.RandomFloat`)) true)))