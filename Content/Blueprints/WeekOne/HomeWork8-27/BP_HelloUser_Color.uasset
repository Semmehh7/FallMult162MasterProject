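; BP_HelloUser_Color is a greeting actor that shows "Hi <username> :)" in a text render component with an animated color.
; BeginPlay sets the text from the platform user name.
; Each Tick calls FunnyColor, which accumulates delta time, samples a vector curve at that time and applies the result as the sRGB text color.
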(event `self.ReceiveBeginPlay`
  (`TextRenderComponent.K2_SetText` (`self.TextRender`) (`|FormatText` "Hi {UserName} :)" (`KismetTextLibrary.Conv_StringToText` (`KismetSystemLibrary.GetPlatformUserName`)))))

(event `self.ReceiveTick`
  (params (DeltaSeconds :type "Float (single-precision)"))
  (`self.FunnyColor` DeltaSeconds))

(fn `FunnyColor`
  (params (`Delta Seconds` :type "Float (double-precision)"))
  (set `self.Delta Seconds` `Delta Seconds`)
  (set `self.Delta Accumulator` (+ (`self.Delta Accumulator`) (`self.Delta Seconds`)))
  (`TextRenderComponent.SetTextRenderColor` (`self.TextRender`) (`KismetMathLibrary.Conv_LinearColorToColor` (`KismetMathLibrary.Conv_VectorToLinearColor` (`CurveVector.GetVectorValue` (`self.FunnyColorCurve`) (`self.Delta Accumulator`))))))

(fn `UserConstructionScript`)