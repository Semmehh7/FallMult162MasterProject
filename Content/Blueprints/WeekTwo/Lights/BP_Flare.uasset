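; BP_Flare is a flare light Blueprint that animates the intensity of its point light over time.
; Tick accumulates delta time, samples a float curve at that elapsed time and scales the result by an Intensity variable to set the light's brightness.
; The elapsed time is never reset or wrapped, so any looping depends on the curve itself.
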(event `self.ReceiveBeginPlay`)

(event `self.ReceiveTick`
  (params (DeltaSeconds :type "Float (single-precision)"))
  (set `self.Delta Seconds` DeltaSeconds)
  (set `self.DeltaTimeAccum` (+ (`self.DeltaTimeAccum`) (`self.Delta Seconds`)))
  (`LightComponent.SetIntensity` (`self.PointLight`) (* (`CurveFloat.GetFloatValue` (`self.Cruve`) (`self.DeltaTimeAccum`)) (`self.Intensity`))))

(fn `UserConstructionScript`)